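; BP_Order is an interactive order machine where the player delivers orders and cooked dishes appear.
; When clicked and overlapped by BP_TopDownCharacter, Tick calls StartDeliveringOrder on the order menu widget and switches input to UI-only.
; OrderNewDish adds to a pending count, which Tick drains by spawning BP_Food at free CookedDishQue slots using offsets from CookedDishLoc.
; That while loop has no exit when every slot is full.
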(event `self.ReceiveBeginPlay`)

(event `self.ReceiveTick`
  (params (DeltaSeconds :type "Float (single-precision)"))
  (bind _returnvalue (> (`self.OrderedDishNum`) 0))
  (`|ExecutionSequence`
    (:`then_0`
      ; 주문 전달하기
      (if (`self.IsUsing?`)
        _
        (elif (and (`self.IsOrderClicked?`) (`self.IsOrderOverlaping?`))
          (set `self.IsUsing?` true)
          (set `self.IsOrderClicked?` false)
          (cast `/Game/PlayerCharacter/Blueprints/BP_TopDownCharacter` (`self.OverlpingActor`))
          (`KismetSystemLibrary.PrintString` "Activate Order Machine")
          (`/Game/UI/WBP_OrderMenu_WashDish.StartDeliveringOrder` (`self.OrderMenuWidgetRef`))
          (bind _asbp_top_down_player_controller (cast `/Game/PlayerCharacter/Blueprints/BP_TopDownPlayerController` (`GameplayStatics.GetPlayerController` 0)))
          (`WidgetBlueprintLibrary.SetInputMode_UIOnlyEx` _asbp_top_down_player_controller null))))
    (:`then_1`
      (if _returnvalue
        (while _returnvalue
          (for (_array_element _array_index) (`self.CookedDish_Que`)
            (if (not _array_element)
              (set `self.OrderedDishNum` (- (`self.OrderedDishNum`) 1))
              (`KismetArrayLibrary.Array_Set` (`self.CookedDish_Que`) _array_index true)
              (`|SpawnActorFromClass` "/Game/Assets/InteractiveActors/BP_Food.BP_Food_C" (`KismetMathLibrary.MakeTransform` (+ (`|GetArrayItem` (`self.CookedDish_Loc`) _array_index) (`self.K2_GetActorLocation`))) "Undefined" "MultiplyWithRoot" null null)
              (break))))))))

(event `self.ReceiveActorOnClicked`
  (params (ButtonPressed :type "Key Structure"))
  (set `self.IsOrderClicked?` true))

(event `self.BoxCollision.OnComponentBeginOverlap`
  (params (OverlappedComponent :type "PrimitiveComponent Object Reference") (OtherActor :type "Actor Object Reference") (OtherComp :type "PrimitiveComponent Object Reference") (OtherBodyIndex :type Integer) (bFromSweep :type Boolean) (SweepResult :type "HitResult Structure (by ref)"))
  (set `self.IsOrderOverlaping?` true)
  (set `self.OverlpingActor` OtherActor))

(event `self.BoxCollision.OnComponentEndOverlap`
  (params (OverlappedComponent :type "PrimitiveComponent Object Reference") (OtherActor :type "Actor Object Reference") (OtherComp :type "PrimitiveComponent Object Reference") (OtherBodyIndex :type Integer))
  (set `self.IsOrderOverlaping?` false)
  (set `self.OverlpingActor` null))

(fn `CheckDishNum`
  (returns (NewParam :type Integer))
  (return (`self.OrderedDishNum`)))

(fn `OrderNewDish`
  (params (NewParam :type Integer))
  (set `self.OrderedDishNum` (+ NewParam (`self.OrderedDishNum`)))
  (return))

(fn `UserConstructionScript`)