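; Clickable restaurant table that seats customers, takes their order and receives served food, branching on the player character's WorkingStatus.
; When idle, a click seats the controller's selected customer in the first empty chair and starts a delayed order, or clears dishes once the guests are gone.
; When delivering, a click moves carried food onto plate points, then after an eating delay hides the food and destroys the customers.
; The table's WBP_CustomerStatus widget shows the order stages.
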(event `self.ReceiveActorOnClicked`
  (params (ButtonPressed :type "Key Structure"))
  (bind _seat (`self.Seat`))
  (bind _havedish_ (`self.HaveDish?`))
  (bind _seat_2 (`self.Seat`))
  (bind _asbp_top_down_character (cast `/Game/PlayerCharacter/Blueprints/BP_TopDownCharacter` (`GameplayStatics.GetPlayerCharacter` 0)))
  (switch `/Game/PlayerCharacter/Blueprints/Enum_PlayerState` (`/Game/PlayerCharacter/Blueprints/BP_TopDownCharacter.WorkingStatus` _asbp_top_down_character)
    (:`NewEnumerator0`
      ; Idle: 손님 좌석 배정, 자리 정리
      (if (`self.IsUsing?`)
        (for _array_element (`self.Seat`)
          (if (`KismetSystemLibrary.IsValid` _array_element)
            (set `self.NoCustomer?` false)))
        (if (`self.NoCustomer?`)
          (for (_array_element_2 _array_index) _havedish_
            (if (`KismetSystemLibrary.IsValid` _array_element_2)
              (bind _asbp_top_down_character_2 (cast `/Game/PlayerCharacter/Blueprints/BP_TopDownCharacter` (`GameplayStatics.GetPlayerCharacter` 0)))
              (bind _pickedplatesnum (`/Game/PlayerCharacter/Blueprints/BP_TopDownCharacter.PickedPlatesNum` _asbp_top_down_character_2))
              (`KismetArrayLibrary.Array_Set` (`/Game/PlayerCharacter/Blueprints/BP_TopDownCharacter.PickedPlates` _asbp_top_down_character_2) _pickedplatesnum _array_element_2)
              (`KismetArrayLibrary.Array_Set` _havedish_ _array_index)
              (set `/Game/PlayerCharacter/Blueprints/BP_TopDownCharacter.PickedPlatesNum` (+ _pickedplatesnum 1) _asbp_top_down_character_2)))
          (set `/Game/PlayerCharacter/Blueprints/BP_TopDownCharacter.WorkingStatus` "NewEnumerator4" _asbp_top_down_character_2))
        (else
          (bind _asbp_top_down_player_controller (cast `/Game/PlayerCharacter/Blueprints/BP_TopDownPlayerController` (`GameplayStatics.GetPlayerController` 0)))
          ;; 좌석 배정
          (bind _asbp_customer (cast `/Game/Assets/NPCs/Customer/BP_Customer` (`/Game/PlayerCharacter/Blueprints/BP_TopDownPlayerController.SelectedActor` _asbp_top_down_player_controller)))
          (for (_array_element_3 _array_index_2) _seat_2
            (if (not (`KismetSystemLibrary.IsValid` _array_element_3))
              (`KismetArrayLibrary.Array_Set` _seat_2 _array_index_2 _asbp_customer)
              (bind _chairtrans (`self.GetChairTransform` _array_index_2))
              (switch `int` _array_index_2
                (:`Default`
                  _)
                (:`0`
                  (`self.K2_AddActorWorldRotation` _asbp_customer (struct :`Yaw` 180.0) false false :!label _label))
                (:`1`
                  (goto _label)))
              (`self.K2_SetActorLocation` _asbp_customer (`KismetMathLibrary.MakeVector` (.x _chairtrans) (.y _chairtrans)) false true)
              (set `/Game/PlayerCharacter/Blueprints/BP_TopDownPlayerController.SelectedActor` null _asbp_top_down_player_controller)
              (set `/Game/Assets/NPCs/Customer/BP_Customer.IsSeated?` true _asbp_customer)
              ;; 배정된 테이블 정보 전달
              (set `/Game/Assets/NPCs/Customer/BP_Customer.Table_WorkingLoc` (`SceneComponent.K2_GetComponentLocation` (`self.WorkingLoc`)) _asbp_customer)
              (set `self.IsUsing?` true)
              (break)))
          (`self.Order`))))
    (:`NewEnumerator3`
      (if (`self.IsUsing?`)
        (bind _asbp_top_down_character_3 (cast `/Game/PlayerCharacter/Blueprints/BP_TopDownCharacter` (`GameplayStatics.GetPlayerCharacter` 0)))
        (bind _pickedfood (`/Game/PlayerCharacter/Blueprints/BP_TopDownCharacter.PickedFood` _asbp_top_down_character_3))
        (for (_array_element_4 _array_index_3) _pickedfood
          (if (`KismetSystemLibrary.IsValid` _array_element_4)
            (for (_array_element_5 _array_index_4) (`self.HaveDish?`)
              (if (not (`KismetSystemLibrary.IsValid` _array_element_5))
                (`KismetArrayLibrary.Array_Set` (`self.HaveDish?`) _array_index_4 _array_element_4)
                (switch `int` _array_index_4
                  (:`0`
                    (`self.K2_SetActorLocation` _array_element_4 (`SceneComponent.K2_GetComponentLocation` (`self.Plate1`)) false false))
                  (:`1`
                    (`self.K2_SetActorLocation` _array_element_4 (`SceneComponent.K2_GetComponentLocation` (`self.Plate2`)) false false))
                  (:`2`
                    (`self.K2_SetActorLocation` _array_element_4 (`SceneComponent.K2_GetComponentLocation` (`self.Plate3`)) false false))
                  (:`3`
                    (`self.K2_SetActorLocation` _array_element_4 (`SceneComponent.K2_GetComponentLocation` (`self.Plate4`)) false false)))
                (`KismetArrayLibrary.Array_Set` _pickedfood _array_index_3)
                (break)))))
        ; 서빙 해줬으니까 음식 요구 그만
        (bind _aswbp_customer_status (cast `/Game/Assets/InteractiveActors/Table/WBP_CustomerStatus` (`WidgetComponent.GetUserWidgetObject` (`self.StatusWidget`))))
        (`/Game/Assets/InteractiveActors/Table/WBP_CustomerStatus.HideUI` _aswbp_customer_status)
        ; 플레이어 양손 가볍게 해주기
        (set `/Game/PlayerCharacter/Blueprints/BP_TopDownCharacter.PickedFoodNum` 0 _asbp_top_down_character_3)
        (set `/Game/PlayerCharacter/Blueprints/BP_TopDownCharacter.WorkingStatus` "NewEnumerator0" _asbp_top_down_character_3)
        ; 식사 시간
        (`KismetSystemLibrary.Delay` 10.0)
        ; 음식 다 먹기
        (for _array_element_6 (`self.HaveDish?`)
          (if (`KismetSystemLibrary.IsValid` _array_element_6)
            (`SceneComponent.SetVisibility` (`/Game/Assets/InteractiveActors/BP_Food.Food` _array_element_6) false false)))
        ; 손님 떠나기
        (for (_array_element_7 _array_index_5) _seat
          (if (`KismetSystemLibrary.IsValid` _array_element_7)
            (`self.K2_DestroyActor` _array_element_7)
            (`KismetArrayLibrary.Array_Set` _seat _array_index_5)))))))

(event `Order`
  ; Idle: 손님 좌석 배정, 자리 정리
  ;; 음식 주문
  (`KismetSystemLibrary.Delay` (`KismetMathLibrary.Conv_IntToDouble` (`KismetMathLibrary.RandomIntegerInRange` 2 4)))
  (bind _aswbp_customer_status (cast `/Game/Assets/InteractiveActors/Table/WBP_CustomerStatus` (`WidgetComponent.GetUserWidgetObject` (`self.StatusWidget`))))
  (`/Game/Assets/InteractiveActors/Table/WBP_CustomerStatus.Decide` _aswbp_customer_status))

(event `self.ReceiveBeginPlay`
  (bind _aswbp_customer_status (cast `/Game/Assets/InteractiveActors/Table/WBP_CustomerStatus` (`WidgetComponent.GetUserWidgetObject` (`self.StatusWidget`))))
  (set `/Game/Assets/InteractiveActors/Table/WBP_CustomerStatus.ParentTable` self _aswbp_customer_status))

(event `PlayerArrivedToGetOrder`
  ; Idle: 손님 좌석 배정, 자리 정리
  ;; 음식 주문
  (bind _aswbp_customer_status (cast `/Game/Assets/InteractiveActors/Table/WBP_CustomerStatus` (`WidgetComponent.GetUserWidgetObject` (`self.StatusWidget`))))
  (`/Game/Assets/InteractiveActors/Table/WBP_CustomerStatus.OrderMenu` _aswbp_customer_status)
  (bind _asbp_top_down_player_controller (cast `/Game/PlayerCharacter/Blueprints/BP_TopDownPlayerController` (`GameplayStatics.GetPlayerController` 0)))
  (`self.EnableInput` _asbp_top_down_player_controller null)
  (bind _asbp_top_down_character (cast `/Game/PlayerCharacter/Blueprints/BP_TopDownCharacter` (`GameplayStatics.GetPlayerCharacter` 0)))
  (set `/Game/PlayerCharacter/Blueprints/BP_TopDownCharacter.WorkingStatus` "NewEnumerator0" _asbp_top_down_character))

(fn `GetChairTransform`
  (params (SeatIndex :type Integer))
  (returns (ChairTrans :type "Vector Structure"))
  (switch `int` SeatIndex
    (:`0`
      (return (`SceneComponent.K2_GetComponentLocation` (`self.Chair1`))))
    (:`1`
      (return (`SceneComponent.K2_GetComponentLocation` (`self.Chair2`))))
    (:`2`
      (return (`SceneComponent.K2_GetComponentLocation` (`self.Chair3`))))
    (:`3`
      (return (`SceneComponent.K2_GetComponentLocation` (`self.Chair4`))))))

(fn `UserConstructionScript`)