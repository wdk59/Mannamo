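; BP_Customer is a customer NPC that the player can click to select for seat assignment.
; When clicked while not seated, it casts the first player controller to BP_TopDownPlayerController and sets itself as that controller's SelectedActor.
; The hit, overlap and tick events do no work, and a debug print of a collision object type is left unconnected.
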(event `self.ReceiveActorOnClicked`
  (params (ButtonPressed :type "Key Structure"))
  (if (not (`self.IsSeated?`))
    ; 좌석 배정
    (bind _asbp_top_down_player_controller (cast `/Game/PlayerCharacter/Blueprints/BP_TopDownPlayerController` (`GameplayStatics.GetPlayerController` 0)))
    (set `/Game/PlayerCharacter/Blueprints/BP_TopDownPlayerController.SelectedActor` self _asbp_top_down_player_controller)))

(event `self.CapsuleComponent.OnComponentHit`
  (params (HitComponent :type "PrimitiveComponent Object Reference") (OtherActor :type "Actor Object Reference") (OtherComp :type "PrimitiveComponent Object Reference") (NormalImpulse :type "Vector Structure") (Hit :type "HitResult Structure (by ref)")))

(event `self.ReceiveTick`
  (params (DeltaSeconds :type "Float (single-precision)"))
  (if true
    _))

(fn `UserConstructionScript`)